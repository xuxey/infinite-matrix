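; BP_Projectile is a shot that destroys enemies and scores a point for the player.
; Each tick it moves its Projectile component along world X by Speed scaled by delta time, without a movement component.
; On overlap it destroys any BP_Enemy and calls AddScore on BP_Player via the player pawn.
; It destroys itself on non-enemy overlaps too, but survives an enemy hit if the player cast fails.
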(event OnComponentBeginOverlap(Projectile)
  (params (OverlappedComponent :type Primitive%20Component%20Object%20Reference) (OtherActor :type Actor%20Object%20Reference) (OtherComp :type Primitive%20Component%20Object%20Reference) (OtherBodyIndex :type Integer) (bFromSweep :type Boolean) (SweepResult :type Hit%20Result%20Structure%20%28by%20ref%29))
  (bind _asbp_enemy (Utilities|Casting|CastToBP_Enemy OtherActor)
    (:then
      (Actor|DestroyActor _asbp_enemy)
      (bind _asbp_player (Utilities|Casting|CastToBP_Player (Game|Player|GetPlayerPawn 0)))
      (Default|AddScore _asbp_player 1))
    (:CastFailed
      _))
  (Actor|DestroyActor))

(event EventBeginPlay)

(event Collision|EventActorBeginOverlap
  (params (OtherActor :type Actor%20Object%20Reference)))

(event EventTick
  (params (DeltaSeconds :type Float%20%28single-precision%29))
  (Transformation|AddWorldOffset (Variables|Default|GetProjectile) (Math|Vector|MakeVector (* DeltaSeconds (Variables|Default|GetSpeed)) 0.0 0.0) false false))

(fn ConstructionScript)